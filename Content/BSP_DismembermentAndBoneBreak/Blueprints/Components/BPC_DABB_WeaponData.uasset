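; Weapon data component for the Dismemberment and Bone Break system that matches weapon animations to the owning character's damage state.
; Initialisation caches the owner's character, bone data and camera plus the active weapon, while events update bone data and the ADS flag.
; The animation getter reads the bone data's damage stage, returns the matching animation-state entry and has the BP_Weapon_Master update its offset.
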(event Custom|DABB_SwitchADS_Client
  (params (bIsADS :type Boolean))
  (Variables|Default|SetbIsADS bIsADS))

(event EventInitialise
  (params (Owning :type F%20Bone%20Break%20Owning%20Structure) (ActiveWeapon :type Actor%20Object%20Reference))
  ;[0.07451 0.1216 0.2706] Set a reference to the OwningCharacter, BoneData, and the ActiveWeapon (Initialised from the EventBeginPlay of the owning character)
  (Variables|SetByInterfaceInteractions|SetOwningCharacter (.character Owning))
  (Variables|SetByInterfaceInteractions|SetOwningBoneData (.bonedata Owning))
  (Variables|SetByInterfaceInteractions|SetActiveWeaponReference ActiveWeapon)
  (Variables|Default|SetPlayerCamera (.thirdpersoncamera Owning)))

(event EventSetWeaponData
  (params (BoneDataComponent :type BPC%20DABB%20Bone%20Data%20Object%20Reference))
  (Variables|SetByInterfaceInteractions|SetOwningBoneData BoneDataComponent))

(fn FDABBGetStateOfDammagefromOwningBoneData
  (bind _owningbonedata (Variables|SetByInterfaceInteractions|GetOwningBoneData))
  ;[0.07451 0.1216 0.2706] Get animationstate from owning player reference so that the correct Animation state can be applied to the weapon
  (Utilities|IsValid (Variables|SetByInterfaceInteractions|GetOwningCharacter)
    (:Is%20Valid
      (Utilities|IsValid _owningbonedata
        (:Is%20Valid
          (Variables|AnimationAffectors|SetStateOfDamageFromBoneData (Variables|/Game/BSP_DismembermentAndBoneBreak/Blueprints/Components/BPC_DABB_BoneData.BPC_DABB_BoneData_C|GetStageOfDamage _owningbonedata))
          (bind _asbp_weapon_master (Utilities|Casting|CastToBP_Weapon_Master (Variables|SetByInterfaceInteractions|GetActiveWeaponReference))
            (:then
              (Default|FDABBUpdateOffset _asbp_weapon_master)
              (return))
            (:CastFailed
              (return))))))
    (:Is%20Not%20Valid
      (return))))

(fn FDABBGetWeaponAnimations
  ;[0.07451 0.1216 0.2706] Update list of animations based on the animation state of ownig character
  (CallFunction|FDABBGetStateOfDammagefromOwningBoneData)
  (for _array_element (Variables|AnimationList|GetST_Owning_Charater_Weapon_Animation_State)
    (Utilities|IsValid (Variables|SetByInterfaceInteractions|GetOwningBoneData)
      (:Is%20Valid
        (for _array_element_2 (.CharacterDamageState (Utilities|Struct|BreakFWeapon_ActionStates _array_element))
          (if (Utilities|Enum|Equal(Enum) _array_element_2 (Variables|/Game/BSP_DismembermentAndBoneBreak/Blueprints/Components/BPC_DABB_BoneData.BPC_DABB_BoneData_C|GetStageOfDamage (Variables|SetByInterfaceInteractions|GetOwningBoneData)))
            (Variables|AnimationList|SetLocalWeaponDataCurentAnimationState _array_element)
            (bind _asbp_weapon_master (Utilities|Casting|CastToBP_Weapon_Master (Variables|SetByInterfaceInteractions|GetActiveWeaponReference))
              (:then
                (Default|FDABBUpdateOffset _asbp_weapon_master)
                (return _array_element))
              (:CastFailed
                (return _array_element)))))))))

(fn GetWeaponData
  (return self))