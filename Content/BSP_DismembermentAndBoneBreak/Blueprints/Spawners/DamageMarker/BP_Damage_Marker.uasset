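; BP_Damage_Marker is a floating damage number actor that shows a damage amount as rising text.
; On BeginPlay it writes DamageToMarker into the DamageFloater text and colors it green, blue or red by damage tier, or destroys itself if the damage is zero.
; A timeline moves the text and its shadow component upward through relative Z offsets, then destroys the actor when finished.
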(event EventBeginPlay
  ;[1 1 1] if No damage registered auto destroy
  (if (not (== (Variables|Default|GetDamageToMarker) 0.0))
    ;[1 1 1] Set Text value from relitive damage
    (Rendering|Components|TextRender|SetText (Variables|Default|GetDamageFloater) (Utilities|Text|ToText(Float) (Variables|Default|GetDamageToMarker) "HalfToEven"))
    ;[1 1 1] Set Color on damage
    (if (<= (Variables|Default|GetDamageToMarker) 5e+01)
      (Rendering|Components|TextRender|SetTextRenderColor (Variables|Default|GetDamageFloater) (Math|Color|MakeColor 0 255 0 1))
      ;[1 1 1] Move the Text up
      (bind _text_float (Timeline|TextFlotationCurve PlayFromStart)
        (:Update
          (Transformation|AddRelativeLocation (Variables|Default|GetDamageFloater) (Math|Vector|MakeVector 0.0 0.0 _text_float) false false)
          (Transformation|AddRelativeLocation (Variables|Default|GetDamageFloaterShadow) (Math|Vector|MakeVector 0.0 0.0 _text_float) false false))
        (:Finished
          (Actor|DestroyActor)))
      (elif (<= (Variables|Default|GetDamageToMarker) 1e+02)
        (Rendering|Components|TextRender|SetTextRenderColor (Variables|Default|GetDamageFloater) (Math|Color|MakeColor 255 0 0 1))
        (Timeline|TextFlotationCurve PlayFromStart)
        (else
          (Rendering|Components|TextRender|SetTextRenderColor (Variables|Default|GetDamageFloater) (Math|Color|MakeColor 0 0 255 1))
          (Timeline|TextFlotationCurve PlayFromStart))))
    (else
      (Actor|DestroyActor))))

(fn ConstructionScript)