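; Game mode for the dismemberment and bone break package that handles session startup and player respawning.
; On BeginPlay, a dedicated server starts a non-LAN session, then on success opens the Preview level with the listen option and caches a SpawnLocation actor.
; ResapwnPlayer waits on a fixed Delay, spawns the supplied character class at the passed transform rather than the cached actor, and has the given controller possess it.
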(event Custom|ResapwnPlayer
  (params (PlayerController :type Player%20Controller%20Object%20Reference) (PlayerCharcter :type Character%20Class%20Reference) (RespawnLocation :type Transform))
  (Utilities|FlowControl|Delay 5.0)
  (bind _returnvalue (Game|SpawnActorfromClass PlayerCharcter RespawnLocation "AdjustIfPossibleButAlwaysSpawn" 0 0))
  (Utilities|IsValid _returnvalue
    (:Is%20Valid
      (Pawn|Possess PlayerController _returnvalue))))

(event EventBeginPlay
  (if (Networking|IsDedicatedServer)
    (|Session (Game|GetPlayerController 0) 0 false
      (:OnSuccess
        (Game|OpenLevel(byName) "Preview" true "?listen")
        (bind _returnvalue (Actor|GetActorOfClass 0))
        (Variables|Default|SetSpawnLocation _returnvalue)))))

(fn ConstructionScript)